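; BP_PlayerPawn is a player pawn that slides its Cube component along local X from input.
; Each Tick, an axis key value times PlayerSpeed is clamped between MinMove and MaxMove and applied as a local offset, without delta-time scaling.
; ChangeMoveDirection overwrites both clamp limits, controlling how far the cube can step in each direction per frame.
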(event `self.ReceiveTick`
  (params (DeltaSeconds :type "Float (single-precision)"))
  ;[1 1 1] PlayerMove
  (`SceneComponent.K2_AddLocalOffset` (`self.Cube`) (`KismetMathLibrary.MakeVector` (`KismetMathLibrary.FClamp` (* (`self.GetInputAxisKeyValue`) (`self.PlayerSpeed`)) (`self.MinMove`) (`self.MaxMove`))) false false))

(fn `ChangeMoveDirection`
  (params (MinMove :type "Float (double-precision)") (MaxMove :type "Float (double-precision)"))
  (set `self.MinMove` MinMove)
  (set `self.MaxMove` MaxMove))

(fn `UserConstructionScript`)