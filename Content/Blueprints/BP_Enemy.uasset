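; BP_Enemy is an opponent that slides its Cube component along Y to follow the ball, like an AI paddle.
; Each Tick it finds the BP_Balls actor and stores its Sphere's relative location in EnemyMoveDirection.
; ChangeMoveDirection then calls MoveComponentTo toward that Y, clamped to a fixed range, with EnemySpeedOverTime as the move duration that sets how quickly it tracks.
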(event `self.ReceiveTick`
  (params (DeltaSeconds :type "Float (single-precision)"))
  (bind _returnvalue (`GameplayStatics.GetActorOfClass` "/Game/Blueprints/BP_Balls.BP_Balls_C"))
  (set `self.EnemyMoveDirection` (`SceneComponent.RelativeLocation` (`/Game/Blueprints/BP_Balls.Sphere` _returnvalue)))
  (`self.ChangeMoveDirection`))

(event `ChangeMoveDirection`
  (bind (_enemymovedirection_x _enemymovedirection_y) (`KismetMathLibrary.BreakVector` (`self.EnemyMoveDirection`)))
  (`KismetSystemLibrary.MoveComponentTo` (`self.Cube`) (`KismetMathLibrary.MakeVector` 0.0 (`KismetMathLibrary.FClamp` _enemymovedirection_y -310.0 310.0)) (struct) false false (`self.EnemySpeedOverTime`)))

(fn `UserConstructionScript`)